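; BP_Projectile is a shot that destroys enemies and awards score to the player.
; Each tick it moves along world X with a swept offset, then raises its speed by a fixed per-frame step up to a cap.
; On sphere overlap it destroys any BP_Enermy and adds a point to BP_Player, then destroys itself.
; Non-enemy overlaps also destroy it, but a failed player cast after a kill leaves it alive.
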(event `self.ReceiveTick`
  (params (DeltaSeconds :type "Float (single-precision)"))
  (`self.K2_AddActorWorldOffset` (`KismetMathLibrary.MakeVector` (* DeltaSeconds (`self.ProjectileSpeed`))) true)
  (`self.IncrementSpeedProjectile`))

(event `self.Sphere.OnComponentBeginOverlap`
  (params (OverlappedComponent :type "PrimitiveComponent Object Reference") (OtherActor :type "Actor Object Reference") (OtherComp :type "PrimitiveComponent Object Reference") (OtherBodyIndex :type Integer) (bFromSweep :type Boolean) (SweepResult :type "HitResult Structure (by ref)"))
  (bind _asbp_enermy (cast `/Game/InfiniteMatrix/Blueprints/BP_Enermy` OtherActor)
    (:`then`
      (`self.K2_DestroyActor` _asbp_enermy)
      (bind _asbp_player (cast `/Game/InfiniteMatrix/Blueprints/BP_Player` (`GameplayStatics.GetPlayerPawn` 0)))
      (`/Game/InfiniteMatrix/Blueprints/BP_Player.IncrementScore` _asbp_player 1))
    (:`CastFailed`
      _))
  (`self.K2_DestroyActor`))

(fn `IncrementSpeedProjectile`
  (set `self.ProjectileSpeed` (`KismetMathLibrary.FMin` (+ (`self.ProjectileSpeed`) 0.25) 4000.0)))

(fn `UserConstructionScript`)